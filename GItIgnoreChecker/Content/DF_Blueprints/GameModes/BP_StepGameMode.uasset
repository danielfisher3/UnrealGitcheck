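; Game mode that sets up a step-based objective and displays it on a spawned UI actor.
; On BeginPlay it finds the actor's WBP_StepVisuals widget, builds a BaseStep with hard-coded placeholder tasks, and pushes its name, description and tasks to the widget.
; Tick runs through a one-second Delay to count elapsed minutes and seconds, which are not passed to the UI.
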(event `self.ReceiveBeginPlay`
  (bind _wbp_step_visuals (`self.WBP Step Visuals`))
  (bind _returnvalue (`|SpawnActorFromClass` (`self.UISpawer`) (`self.GetTransform`) "Undefined" "MultiplyWithRoot" null null))
  (bind _output_get (set `self.ActorWithUI` _returnvalue))
  (bind _output_get_2 (set `self.WidgetComponent` (`self.GetComponentByClass` _output_get "/Script/UMG.WidgetComponent")))
  (bind _output_get_3 (set `self.Widget` (`WidgetComponent.GetWidget` _output_get_2)))
  (bind _aswbp_step_visuals (cast `/Game/DF_Blueprints/UI/WBP_StepVisuals` _output_get_3))
  (set `self.WBP Step Visuals` _aswbp_step_visuals)
  (bind _returnvalue_2 (`|GenericCreateObject` self "/Script/GItIgnoreChecker.BaseStep"))
  (bind _output_get_4 (set `self.CurrentStepRef` _returnvalue_2))
  (`BaseStep.SetupNumOfTasks` _output_get_4 2)
  (`BaseStep.SetStepDetails` _output_get_4 "Step 1" "Greatness Awaits")
  (`BaseStep.SetupStepTask` _output_get_4 0 "Go To Pie")
  (`BaseStep.SetupStepTask` _output_get_4 1 "Eat Pie")
  (`/Game/DF_Blueprints/UI/WBP_StepVisuals.SetStepName` _wbp_step_visuals (`KismetTextLibrary.Conv_StringToText` (`BaseStep.StepName` _output_get_4)))
  (`/Game/DF_Blueprints/UI/WBP_StepVisuals.SetStepDescription` _wbp_step_visuals (`KismetTextLibrary.Conv_StringToText` (`BaseStep.StepDescription` _output_get_4)))
  (for _array_element (`BaseStep.StepTasks` (`self.CurrentStepRef`))
    (`/Game/DF_Blueprints/UI/WBP_StepVisuals.SetTaskDecription` (`self.WBP Step Visuals`) (`KismetTextLibrary.Conv_StringToText` (`.StepTaskDescription` (break `StepTask` _array_element))))
    (`VerticalBox.AddChildToVerticalBox` (`/Game/DF_Blueprints/UI/WBP_StepVisuals.Box` (`self.WBP Step Visuals`)) null)))

(event `self.ReceiveTick`
  (params (DeltaSeconds :type "Float (single-precision)"))
  (`KismetSystemLibrary.Delay` 1.0)
  (set `self.TimeSecs` (+ (`self.TimeSecs`) 1))
  (if (> (`self.TimeSecs`) 59)
    (set `self.TimeMin` (+ (`self.TimeMin`) 1))
    (set `self.TimeSecs` 0)))

(fn `UserConstructionScript`)